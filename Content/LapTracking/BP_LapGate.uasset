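; BP_LapGate is a numbered gate actor for lap tracking.
; When its Cube is overlapped, the server looks for a BP_LapGateUser component on the other actor and passes it the gate number and last-gate value through EnterGate.
; If EnterGate succeeds, ClientEnterGate spawns particle emitters attached to the left and right sides of the gate.
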(event `self.Cube.OnComponentBeginOverlap`
  (params (OverlappedComponent :type "PrimitiveComponent Object Reference") (OtherActor :type "Actor Object Reference") (OtherComp :type "PrimitiveComponent Object Reference") (OtherBodyIndex :type Integer) (bFromSweep :type Boolean) (SweepResult :type "HitResult Structure (by ref)"))
  (bind _returnvalue (`self.GetComponentByClass` OtherActor "/Game/LapTracking/BP_LapGateUser.BP_LapGateUser_C"))
  (if (`KismetSystemLibrary.IsServer`)
    (if (!= _returnvalue null)
      (bind _correctgate (`/Game/LapTracking/BP_LapGateUser.EnterGate` _returnvalue (`self.GateNumber`) (`self.LastGate`)))
      (if _correctgate
        (`self.ClientEnterGate`)))))

(event `ClientEnterGate`
  (`|ExecutionSequence`
    (:`then_0`
      (`GameplayStatics.SpawnEmitterAttached` (`self.Particles`) (`self.LeftParticles`)))
    (:`then_1`
      (`GameplayStatics.SpawnEmitterAttached` (`self.Particles`) (`self.RightParticles`)))))

(fn `UserConstructionScript`)